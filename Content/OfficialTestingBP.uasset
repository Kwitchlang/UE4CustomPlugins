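; Test Blueprint that applies physics presets from the ListofPhysicsPresets data table in its construction script.
; It looks up the row selected in the PhysicsPresets handle and, unless that row's Dontoveride flag is set, copies its name, gravity and projectile speed into PhysicsData.
; After copying, it resets the handle to the table's second row name.
; The SaveTopreset event is an empty stub.
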(event `Save To preset`)

(fn `UserConstructionScript`
  (bind (_physics_presets_datatable _physics_presets_rowname) (break `DataTableRowHandle` (`self.Physics Presets`)))
  (bind _returnvalue (`|GetDataTableRow` "/CustomUtilities/TestFolder/ListofPhysicsPresets.ListofPhysicsPresets" _physics_presets_rowname)
    (:`then`
      (if (not (`.Dontoveride_8_49ACA82E43BD0A14BF35A98D5F773CE5` (break `/CustomUtilities/TestFolder/PhysicspresetTemplates` _returnvalue)))
        (`|VariableSetRef` (`self.Physics Data`) (make `/CustomUtilities/TestFolder/PhysicsPresetData` (`KismetStringLibrary.Conv_NameToString` _physics_presets_rowname) (break `/CustomUtilities/TestFolder/PhysicspresetTemplates` _returnvalue) (`.ProjectileSpeed_6_40C4124245F7BBBDDD11F99C2A4E6AC6` (break `/CustomUtilities/TestFolder/PhysicspresetTemplates` _returnvalue))))
        (bind _outrownames (`DataTableFunctionLibrary.GetDataTableRowNames` _physics_presets_datatable))
        (set `self.Physics Presets` (make `DataTableRowHandle` "/CustomUtilities/TestFolder/ListofPhysicsPresets.ListofPhysicsPresets" (`|GetArrayItem` _outrownames 1)))))))