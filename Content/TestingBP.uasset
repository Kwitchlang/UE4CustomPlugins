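; Test Blueprint that exercises an advanced button helper and a value-comparison helper through debug prints.
; The K key feeds press and release into advancedButtonConfiguration, which Tick updates, and prints down or up for under- and over-threshold results.
; The construction script prints TestValueDirection's comparison to the previous frame, leaving a CheckValueDirection call disconnected.
; BeginPlay looks up the Blaster row in the Sockets table without using it.
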(event `self.ReceiveBeginPlay`
  (`|GetDataTableRow` "/CustomUtilities/Libraries/DataTables/Sockets.Sockets" "Blaster"))

(event `Key|K`
  (params (Key :type "Key Structure"))
  (:`Pressed`
    (bind _is_button_down_or_released (`/CustomUtilities/Libraries/CustomMacroLibrary.Advanced Button Configuration` true Key (stale `self.ReceiveTick` DeltaSeconds) 0 false true :!label _label)
      (:`Under Threshold`
        (if _is_button_down_or_released
          (`KismetSystemLibrary.PrintString` "Under threshold DOWN")
          (else
            (`KismetSystemLibrary.PrintString` "Under threshold Up"))))
      (:`Over Threshold`
        (if _is_button_down_or_released
          (`KismetSystemLibrary.PrintString` "Over  threshold DOWN")
          (else
            (`KismetSystemLibrary.PrintString` "Over  threshold UP"))))))
  (:`Released`
    (goto _label :!via `Button Released`)))

(event `self.ReceiveTick`
  (params (DeltaSeconds :type "Float (single-precision)"))
  (`|ExecutionSequence`
    (:`then_0`
      (goto _label :!via `Event Tick`))))

(fn `UserConstructionScript`
  (bind _newparam (`/CustomUtilities/Libraries/CustomFunctionLibrary.Compare Value to previous frame` (`self.Test value Direction`)))
  (`KismetSystemLibrary.PrintString` (`KismetStringLibrary.Conv_BoolToString` _newparam)))